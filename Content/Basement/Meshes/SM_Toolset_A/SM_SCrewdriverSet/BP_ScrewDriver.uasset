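; BP_ScrewDriver is a modular screwdriver prop from a basement toolset, assembled from interchangeable head and body meshes.
; The construction script switches on SelectHEAD to set one of three head meshes (PLAT, CRUCI, THORX).
; It also switches on SelectBODY to set one of four body meshes.
; The event graph holds only disabled default events, so it has no runtime logic.
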(event EventBeginPlay)

(event Collision|EventActorBeginOverlap
  (params (OtherActor :type Actor%20Object%20Reference)))

(event EventTick
  (params (DeltaSeconds :type Float%20%28single-precision%29)))

(fn ConstructionScript
  (bind _body (Variables|Default|GetBODY))
  (bind _head (Variables|Default|GetHEAD))
  (switch Utilities|FlowControl|Switch|SwitchonEN_HEADSCREWDRIVER (Variables|Default|GetSelect_HEAD)
    (:NewEnumerator0
      (Components|StaticMesh|SetStaticMesh _head (Variables|Default|GetHEAD_F)))
    (:NewEnumerator1
      (Components|StaticMesh|SetStaticMesh _head (Variables|Default|GetHEAD_C)))
    (:NewEnumerator2
      (Components|StaticMesh|SetStaticMesh _head (Variables|Default|GetHEAD_T))))
  (switch Utilities|FlowControl|Switch|SwitchonEN_BODYSCREWDRIVER (Variables|Default|GetSelect_BODY)
    (:NewEnumerator0
      (Components|StaticMesh|SetStaticMesh _body (Variables|Default|GetBODY_0)))
    (:NewEnumerator1
      (Components|StaticMesh|SetStaticMesh _body (Variables|Default|GetBODY_1)))
    (:NewEnumerator2
      (Components|StaticMesh|SetStaticMesh _body (Variables|Default|GetBODY_2)))
    (:NewEnumerator3
      (Components|StaticMesh|SetStaticMesh _body (Variables|Default|GetBODY_3)))))