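; Interactable shake actor that toggles a looping shake on its root when Interac fires, restoring the transform saved at BeginPlay on the next call.
; STYLE flags select location or rotation axes, though the RotZ flag calls the LocZ shake.
; Paired timelines ping-pong each axis between positive and negative offsets, scaled by amplitude and frequency multipliers.
; Each update resets the other two axes to base, so same-type shakes override each other.
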(event Custom|SHAKE_LOC_Y
  (bind _defaultsceneroot (Variables|Default|GetDefaultSceneRoot))
  (bind _defaultsceneroot_2 (Variables|Default|GetDefaultSceneRoot))
  (bind _offsetloc_y (Variables|LOCY|GetOffsetLoc_Y))
  (bind _offsetlocymultiplier (Variables|LOCY|GetOffsetLocYMultiplier))
  (bind _basepos (Variables|Default|GetBasePos))
  (bind _returnvalue (Transformation|GetWorldLocation _defaultsceneroot_2))
  (bind _returnvalue_2 (* _offsetloc_y _offsetlocymultiplier))
  ;[1 0.1022 0] LOCATION
  ;;[1 1 1] Y
  (Components|Timeline|SetPlayRate (Variables|Default|GetTIME_LOCATION_Y) (Variables|LOCY|GetFrequenceLocYMultiplier))
  (bind _newtrack_0 (Timeline|TIME_LOCATION_Y PlayFromStart)
    (:Update
      (Transformation|SetWorldLocation _defaultsceneroot (Math|Vector|MakeVector (.x _basepos) (Math|Float|Lerp (.y _returnvalue) (+ (.y _basepos) _returnvalue_2) _newtrack_0) (.z _basepos)) false false))
    (:Finished
      (bind _newtrack_0_2 (Timeline|TIME_RETURN_LOC_Y PlayFromStart)
        (:Update
          (Transformation|SetWorldLocation _defaultsceneroot (Math|Vector|MakeVector (.x _basepos) (Math|Float|Lerp (.y _returnvalue) (+ (.y _basepos) (* _returnvalue_2 -1.0)) _newtrack_0_2) (.z _basepos)) false false))
        (:Finished
          (Timeline|TIME_LOCATION_Y PlayFromStart))))))

(event Custom|SHAKE_LOC_X
  (bind _offsetloc_x (Variables|LOCX|GetOffsetLoc_X))
  (bind _basepos (Variables|Default|GetBasePos))
  (bind _defaultsceneroot (Variables|Default|GetDefaultSceneRoot))
  (bind _defaultsceneroot_2 (Variables|Default|GetDefaultSceneRoot))
  (bind _offsetlocxmultiplier (Variables|LOCX|GetOffsetLocXMultiplier))
  (bind _returnvalue (Transformation|GetWorldLocation _defaultsceneroot_2))
  (bind _returnvalue_2 (* _offsetloc_x _offsetlocxmultiplier))
  ;[1 0.1022 0] LOCATION
  ;;[1 1 1] X
  (Components|Timeline|SetPlayRate (Variables|Default|GetTIME_RETURN_LOCATION_X) (Variables|LOCX|GetFrequenceLocXMultiplier))
  (bind _newtrack_0 (Timeline|TIME_LOCATION_X PlayFromStart)
    (:Update
      (Transformation|SetWorldLocation _defaultsceneroot (Math|Vector|MakeVector (Math|Float|Lerp (.x _returnvalue) (+ (.x _basepos) _returnvalue_2) _newtrack_0) (.y _basepos) (.z _basepos)) false false))
    (:Finished
      (bind _newtrack_0_2 (Timeline|TIME_RETURN_LOCATION_X PlayFromStart)
        (:Update
          (Transformation|SetWorldLocation _defaultsceneroot (Math|Vector|MakeVector (Math|Float|Lerp (.x _returnvalue) (+ (.x _basepos) (* _returnvalue_2 -1.0)) _newtrack_0_2) (.y _basepos) (.z _basepos)) false false))
        (:Finished
          (Timeline|TIME_LOCATION_X PlayFromStart))))))

(event Custom|SHAKE_ROT_Z
  (bind _offsetrot_z (Variables|ROTZ|GetOffsetRot_Z))
  (bind _offsetrotzmultiplier (Variables|ROTZ|GetOffsetRotZMultiplier))
  (bind _base_rotation (Variables|Default|GetBase%20Rotation))
  (bind _defaultsceneroot (Variables|Default|GetDefaultSceneRoot))
  (bind _returnvalue (Transformation|GetWorldRotation _defaultsceneroot))
  (bind _returnvalue_2 (* _offsetrot_z _offsetrotzmultiplier))
  ;[0 0.1496 1] ROTATION
  ;;[0 1 0.2184] Z
  (Components|Timeline|SetPlayRate (Variables|Default|GetTIME_RETURN_ROT_Z) (Variables|ROTZ|GetFrequenceRotZMultiplier))
  (bind _newtrack_0 (Timeline|TIME_ROTATION_Z PlayFromStart)
    (:Update
      (Transformation|SetWorldRotation (Variables|Default|GetDefaultSceneRoot) (Math|Rotator|MakeRotator (.roll _base_rotation) (.pitch _base_rotation) (Math|Float|Lerp (.yaw _returnvalue) (+ (.yaw _base_rotation) _returnvalue_2) _newtrack_0)) false false))
    (:Finished
      (bind _newtrack_0_2 (Timeline|TIME_RETURN_ROT_Z PlayFromStart)
        (:Update
          (Transformation|SetWorldRotation (Variables|Default|GetDefaultSceneRoot) (Math|Rotator|MakeRotator (.roll _base_rotation) (.pitch _base_rotation) (Math|Float|Lerp (.yaw _returnvalue) (+ (* _returnvalue_2 -1.0) (.yaw _base_rotation)) _newtrack_0_2)) false false))
        (:Finished
          (Timeline|TIME_ROTATION_Z PlayFromStart))))))

(event Custom|SHAKE_ROT_Y
  (bind _base_rotation (Variables|Default|GetBase%20Rotation))
  (bind _defaultsceneroot (Variables|Default|GetDefaultSceneRoot))
  (bind _offsetrot_y (Variables|ROTY|GetOffsetRot_Y))
  (bind _offsetrotymultiplier (Variables|ROTY|GetOffsetRotYMultiplier))
  (bind _base_rotation_2 (Variables|Default|GetBase%20Rotation))
  (bind _returnvalue (Transformation|GetWorldRotation _defaultsceneroot))
  (bind _returnvalue_2 (* _offsetrot_y _offsetrotymultiplier))
  ;[0 0.1496 1] ROTATION
  ;;[1 1 1] Y
  (Components|Timeline|SetPlayRate (Variables|Default|GetTIME_RETURN_ROT_Y) (Variables|ROTY|GetFrequenceRotYMultiplier))
  (bind _newtrack_0 (Timeline|TIME_ROTATION_Y PlayFromStart)
    (:Update
      (Transformation|SetWorldRotation _defaultsceneroot (Math|Rotator|MakeRotator (.roll _base_rotation_2) (Math|Float|Lerp (.pitch _returnvalue) (+ (.pitch _base_rotation_2) _returnvalue_2) _newtrack_0) (.yaw _base_rotation_2)) false false))
    (:Finished
      (bind _newtrack_0_2 (Timeline|TIME_RETURN_ROT_Y PlayFromStart)
        (:Update
          (Transformation|SetWorldRotation _defaultsceneroot (Math|Rotator|MakeRotator (.roll _base_rotation) (Math|Float|Lerp (.pitch _returnvalue) (+ (* _returnvalue_2 -1.0) (.pitch _base_rotation)) _newtrack_0_2) (.yaw _base_rotation)) false false))
        (:Finished
          (Timeline|TIME_ROTATION_Y PlayFromStart))))))

(event Custom|SHAKE_ROT_X
  (bind _base_rotation (Variables|Default|GetBase%20Rotation))
  (bind _defaultsceneroot (Variables|Default|GetDefaultSceneRoot))
  (bind _offsetrot_x (Variables|ROTX|GetOffsetRot_X))
  (bind _offsetrotxmultiplier (Variables|ROTX|GetOffsetRotXMultiplier))
  (bind _returnvalue (Transformation|GetWorldRotation _defaultsceneroot))
  (bind _returnvalue_2 (* _offsetrot_x _offsetrotxmultiplier))
  ;[0 0.1496 1] ROTATION
  ;;[1 1 1] X
  (Components|Timeline|SetPlayRate (Variables|Default|GetTIME_ROTATION_X) (Variables|ROTX|GetFrequence_RotXMultiplier))
  (bind _newtrack_0 (Timeline|TIME_ROTATION_X PlayFromStart)
    (:Update
      (Transformation|SetWorldRotation (Variables|Default|GetDefaultSceneRoot) (Math|Rotator|MakeRotator (Math|Float|Lerp (.roll _returnvalue) (+ (.roll _base_rotation) _returnvalue_2) _newtrack_0) (.pitch _base_rotation) (.yaw _base_rotation)) false false))
    (:Finished
      (bind _newtrack_0_2 (Timeline|TIME_RETURN_ROT_X PlayFromStart)
        (:Update
          (Transformation|SetWorldRotation (Variables|Default|GetDefaultSceneRoot) (Math|Rotator|MakeRotator (Math|Float|Lerp (.roll _returnvalue) (+ (* _returnvalue_2 -1.0) (.roll _base_rotation)) _newtrack_0_2) (.pitch _base_rotation) (.yaw _base_rotation)) false false))
        (:Finished
          (Timeline|TIME_ROTATION_X PlayFromStart))))))

(event Custom|ResetPos
  (bind _defaultsceneroot (Variables|Default|GetDefaultSceneRoot))
  ;[1 1 1] STOP SYSTEM
  (Transformation|SetWorldLocation _defaultsceneroot (Variables|Default|GetBasePos) false false)
  (Transformation|SetWorldRotation _defaultsceneroot (Variables|Default|GetBase%20Rotation) false false)
  (Variables|Default|SetSHAKING? false)
  (Audio|Components|Audio|Stop (Variables|Default|GetTIME_RETURN_LOC_Z)))

(event Custom|SHAKE_LOC_Z
  (bind _basepos (Variables|Default|GetBasePos))
  (bind _defaultsceneroot (Variables|Default|GetDefaultSceneRoot))
  (bind _offsetloc_z (Variables|LOCZ|GetOffsetLoc_Z))
  (bind _offsetloczmultiplier (Variables|LOCZ|GetOffsetLocZMultiplier))
  (bind _defaultsceneroot_2 (Variables|Default|GetDefaultSceneRoot))
  (bind _returnvalue (Transformation|GetWorldLocation _defaultsceneroot))
  (bind _returnvalue_2 (* _offsetloc_z _offsetloczmultiplier))
  ;[1 0.1022 0] LOCATION
  ;;[0 1 0.2184] Z
  (Components|Timeline|SetPlayRate (Variables|Default|GetTIME_RETURN_LOC_Z) (Variables|LOCZ|GetFrequenceLocZMultiplier))
  (bind _newtrack_0 (Timeline|TIME_LOCATION_Z PlayFromStart)
    (:Update
      (Transformation|SetWorldLocation _defaultsceneroot_2 (Math|Vector|MakeVector (.x _basepos) (.y _basepos) (Math|Float|Lerp (.z _returnvalue) (+ (.z _basepos) _returnvalue_2) _newtrack_0)) false false))
    (:Finished
      (bind _newtrack_0_2 (Timeline|TIME_RETURN_LOC_Z PlayFromStart)
        (:Update
          (Transformation|SetWorldLocation _defaultsceneroot_2 (Math|Vector|MakeVector (.x _basepos) (.y _basepos) (Math|Float|Lerp (.z _returnvalue) (+ (.z _basepos) (* _returnvalue_2 -1.0)) _newtrack_0_2)) false false))
        (:Finished
          (Timeline|TIME_LOCATION_Z PlayFromStart))))))

(event EventBeginPlay
  (bind _defaultsceneroot (Variables|Default|GetDefaultSceneRoot))
  (Variables|Default|SetBasePos (Transformation|GetWorldLocation _defaultsceneroot))
  (Variables|Default|SetBase%20Rotation (Transformation|GetWorldRotation _defaultsceneroot)))

(event EventInterac
  ;[1 1 1] CHOOSE STYLE SHAKING
  (if (not (Variables|Default|GetSHAKING?))
    (if (Variables|ChooseAxeShaking|GetSTYLE_Shake_Loc_X?)
      (CallFunction|SHAKELOCX))
    (if (Variables|ChooseAxeShaking|GetSTYLE_Shake_Rot_X?)
      (CallFunction|SHAKEROTX))
    (if (Variables|ChooseAxeShaking|GetSTYLE_Shake_Loc_Y?)
      (CallFunction|SHAKELOCY))
    (if (Variables|ChooseAxeShaking|GetSTYLE_Shake_Rot_Y?)
      (CallFunction|SHAKEROTY))
    (if (Variables|ChooseAxeShaking|GetSTYLE_Shake_Loc_Z)
      (CallFunction|SHAKELOCZ))
    (if (Variables|ChooseAxeShaking|GetSTYLE_Shake_Rot_Z)
      (CallFunction|SHAKELOCZ))
    (Variables|Default|SetSHAKING? true)
    (Development|PrintString "Go Shake")
    (else
      (CallFunction|ResetPos))))

(fn ConstructionScript)