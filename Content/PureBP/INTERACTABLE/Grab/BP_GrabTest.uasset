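; BP_GrabTest is a test interactable physics cube that the first-person player can target, pick up and drop.
; LookingatYou highlights it on the player's HUD, using a retriggerable delay to clear the target once the calls stop.
; Grab disables physics and collision and attaches the cube to the camera; if FACABLE, chained timelines move then rotate it to the FacingZone.
; Grabbing again or pressing IA_INTERACT while held detaches it and restores physics.
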(event Input|EnhancedActionEvents|EnhancedInputActionIA_INTERACT
  (params (ActionValue :type Boolean) (ElapsedSeconds :type Float%20%28double-precision%29) (TriggeredSeconds :type Float%20%28double-precision%29) (InputAction :type Input%20Action%20Object%20Reference :default "/Game/FirstPerson/Input/Actions/IA_INTERACT.IA_INTERACT"))
  (bind _cube (Variables|Default|GetCube))
  (:Triggered
    (if (Variables|Default|GetGrabbed?)
      (Audio|Components|Audio|Stop (Variables|Default|GetTimeForApproach))
      (Variables|/Game/FirstPerson/Blueprints/BP_FirstPersonCharacter.BP_FirstPersonCharacter_C|SetGrabbed? (Variables|Default|GetAs%20BP%20First%20Person%20Character) false)
      (Collision|SetCollisionEnabled _cube "QueryAndPhysics")
      (Physics|SetSimulatePhysics _cube true)
      (Transformation|DetachFromComponent (Variables|Default|GetCube) "KeepWorld" "KeepWorld" "KeepRelative" true)
      (Variables|Default|SetGrabbed? false)
      (Input|DisableInput (Game|GetPlayerController 0)))))

(event EventBeginPlay
  (bind _asbp_first_person_character (CallFunction|GetPlayer))
  (Variables|Default|SetAs%20BP%20First%20Person%20Character _asbp_first_person_character))

(event Collision|EventActorBeginOverlap
  (params (OtherActor :type Actor%20Object%20Reference)))

(event EventLookingatYou
  (bind _as_bp_first_person_character (Variables|Default|GetAs%20BP%20First%20Person%20Character))
  (bind _main_hud (Variables|/Game/FirstPerson/Blueprints/BP_FirstPersonCharacter.BP_FirstPersonCharacter_C|GetMain_HUD _as_bp_first_person_character))
  (if (not (Variables|Default|GetCurrentLook?))
    (Variables|Default|SetCurrentLook? true)
    (Default|SeeTarget _main_hud "/Engine/EditorMaterials/Anchor.Anchor")
    (else
      (Utilities|FlowControl|RetriggerableDelay 0.05)
      (Variables|Default|SetCurrentLook? false)
      (Default|ResetMire _main_hud))))

(event EventGrab
  (bind _as_bp_first_person_character (Variables|Default|GetAs%20BP%20First%20Person%20Character))
  (bind _cube (Variables|Default|GetCube))
  (bind _as_bp_first_person_character_2 (Variables|Default|GetAs%20BP%20First%20Person%20Character))
  (bind _cube_2 (Variables|Default|GetCube))
  (bind _cube_3 (Variables|Default|GetCube))
  (bind _facingzone (Variables|/Game/FirstPerson/Blueprints/BP_FirstPersonCharacter.BP_FirstPersonCharacter_C|GetFacingZone _as_bp_first_person_character))
  (if (not (Variables|Default|GetGrabbed?))
    (if (Variables|Default|GetCurrentLook?)
      (Variables|/Game/FirstPerson/Blueprints/BP_FirstPersonCharacter.BP_FirstPersonCharacter_C|SetGrabbed? _as_bp_first_person_character_2 true)
      (Physics|SetSimulatePhysics _cube_2 false)
      (Collision|SetCollisionEnabled _cube_2 "NoCollision")
      (bind _asbp_first_person_character (CallFunction|GetPlayer))
      (Transformation|AttachComponentToComponent (Variables|Default|GetCube) (Variables|/Game/FirstPerson/Blueprints/BP_FirstPersonCharacter.BP_FirstPersonCharacter_C|GetFirstPersonCamera _asbp_first_person_character) "None" "KeepWorld" "KeepWorld" "KeepWorld" true)
      (Variables|Default|SetGrabbed? true)
      (Input|EnableInput (Game|GetPlayerController 0))
      (if (Variables|Default|GetFACABLE?)
        (bind _newtrack_0 (Timeline|TimeForApproach PlayFromStart)
          (:Update
            (Transformation|SetWorldLocation _cube (Math|Vector|Lerp(Vector) (Transformation|GetWorldLocation _cube) (Transformation|GetWorldLocation _facingzone) _newtrack_0) false false))
          (:Finished
            (bind _newtrack_0_2 (Timeline|Timeline_0 PlayFromStart)
              (:Update
                (Transformation|SetRelativeRotation _cube (Math|Rotator|Lerp(Rotator) (Variables|/Script/Engine.SceneComponent|GetRelativeRotation (Variables|Default|GetCube)) (Variables|/Script/Engine.SceneComponent|GetRelativeRotation _facingzone) _newtrack_0_2) false false)))))))
    (else
      (Variables|/Game/FirstPerson/Blueprints/BP_FirstPersonCharacter.BP_FirstPersonCharacter_C|SetGrabbed? _as_bp_first_person_character_2 false)
      (Collision|SetCollisionEnabled _cube_3 "QueryAndPhysics")
      (Physics|SetSimulatePhysics _cube_3 true)
      (Transformation|DetachFromComponent (Variables|Default|GetCube) "KeepWorld" "KeepWorld" "KeepRelative" true)
      (Variables|Default|SetGrabbed? false)
      (Input|DisableInput (Game|GetPlayerController 0)))))

(fn ConstructionScript)