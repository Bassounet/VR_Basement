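; VR keypad puzzle that generates a random four-digit code on BeginPlay, displays it, and quits the game after it is solved.
; VRPawn DetectZone overlaps press digit buttons with a debounced nudge, blue flash and beep, appending to an entry that clears past four digits.
; The verify button compares and clears the entry.
; A match starts a timed countdown of pitched beeps and yellow flashes, ending in rapid red flashes before quitting.
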(event OnComponentBeginOverlap(Box_7)
  (params (OverlappedComponent :type Primitive%20Component%20Object%20Reference) (OtherActor :type Actor%20Object%20Reference) (OtherComp :type Primitive%20Component%20Object%20Reference) (OtherBodyIndex :type Integer) (bFromSweep :type Boolean) (SweepResult :type Hit%20Result%20Structure%20%28by%20ref%29))
  (bind _asvrpawn (Utilities|Casting|CastToVRPawn OtherActor))
  (if (== (Variables|/Game/VRTemplate/Blueprints/VRPawn.VRPawn_C|GetDetectZone _asvrpawn) OtherComp)
    (if (not (Variables|Default|GetTapped?))
      (Variables|Default|SetTapped? true)
      (CallFunction|Tap (Variables|Default|Get7))
      (Variables|Default|SetCurrent%20Code (Utilities|String|Append (Variables|Default|GetCurrent%20Code) "7"))
      (Audio|PlaySound2D "/Game/SND/Bip_Cue.Bip_Cue" 1.0 1.0 0.0 0 0)
      (CallFunction|Bip)
      (if (> (Utilities|String|Len (Variables|Default|GetCurrent%20Code)) 4)
        (Variables|Default|SetCurrent%20Code "")))))

(event OnComponentBeginOverlap(Box_0)
  (params (OverlappedComponent :type Primitive%20Component%20Object%20Reference) (OtherActor :type Actor%20Object%20Reference) (OtherComp :type Primitive%20Component%20Object%20Reference) (OtherBodyIndex :type Integer) (bFromSweep :type Boolean) (SweepResult :type Hit%20Result%20Structure%20%28by%20ref%29))
  (bind _asvrpawn (Utilities|Casting|CastToVRPawn OtherActor))
  (if (== (Variables|/Game/VRTemplate/Blueprints/VRPawn.VRPawn_C|GetDetectZone _asvrpawn) OtherComp)
    (if (not (Variables|Default|GetTapped?))
      (Variables|Default|SetTapped? true)
      (CallFunction|Tap (Variables|Default|Get0))
      (Variables|Default|SetCurrent%20Code (Utilities|String|Append (Variables|Default|GetCurrent%20Code) "0"))
      (Audio|PlaySound2D "/Game/SND/Bip_Cue.Bip_Cue" 1.0 1.0 0.0 0 0)
      (CallFunction|Bip)
      (if (> (Utilities|String|Len (Variables|Default|GetCurrent%20Code)) 4)
        (Variables|Default|SetCurrent%20Code "")))))

(event OnComponentBeginOverlap(Box)
  (params (OverlappedComponent :type Primitive%20Component%20Object%20Reference) (OtherActor :type Actor%20Object%20Reference) (OtherComp :type Primitive%20Component%20Object%20Reference) (OtherBodyIndex :type Integer) (bFromSweep :type Boolean) (SweepResult :type Hit%20Result%20Structure%20%28by%20ref%29))
  (CallFunction|VerifyBtnHit OtherComp OtherActor)
  (CallFunction|Tap (Variables|Default|GetVERIFY%20BTN))
  (CallFunction|Verify))

(event OnComponentBeginOverlap(Box_8)
  (params (OverlappedComponent :type Primitive%20Component%20Object%20Reference) (OtherActor :type Actor%20Object%20Reference) (OtherComp :type Primitive%20Component%20Object%20Reference) (OtherBodyIndex :type Integer) (bFromSweep :type Boolean) (SweepResult :type Hit%20Result%20Structure%20%28by%20ref%29))
  (bind _asvrpawn (Utilities|Casting|CastToVRPawn OtherActor))
  (if (== (Variables|/Game/VRTemplate/Blueprints/VRPawn.VRPawn_C|GetDetectZone _asvrpawn) OtherComp)
    (if (not (Variables|Default|GetTapped?))
      (Variables|Default|SetTapped? true)
      (CallFunction|Tap (Variables|Default|Get8))
      (Variables|Default|SetCurrent%20Code (Utilities|String|Append (Variables|Default|GetCurrent%20Code) "8"))
      (Audio|PlaySound2D "/Game/SND/Bip_Cue.Bip_Cue" 1.0 1.0 0.0 0 0)
      (CallFunction|Bip)
      (if (> (Utilities|String|Len (Variables|Default|GetCurrent%20Code)) 4)
        (Variables|Default|SetCurrent%20Code "")))))

(event OnComponentBeginOverlap(Box_6)
  (params (OverlappedComponent :type Primitive%20Component%20Object%20Reference) (OtherActor :type Actor%20Object%20Reference) (OtherComp :type Primitive%20Component%20Object%20Reference) (OtherBodyIndex :type Integer) (bFromSweep :type Boolean) (SweepResult :type Hit%20Result%20Structure%20%28by%20ref%29))
  (bind _asvrpawn (Utilities|Casting|CastToVRPawn OtherActor))
  (if (== (Variables|/Game/VRTemplate/Blueprints/VRPawn.VRPawn_C|GetDetectZone _asvrpawn) OtherComp)
    (if (not (Variables|Default|GetTapped?))
      (Variables|Default|SetTapped? true)
      (CallFunction|Tap (Variables|Default|Get6))
      (Variables|Default|SetCurrent%20Code (Utilities|String|Append (Variables|Default|GetCurrent%20Code) "6"))
      (Audio|PlaySound2D "/Game/SND/Bip_Cue.Bip_Cue" 1.0 1.0 0.0 0 0)
      (CallFunction|Bip)
      (if (> (Utilities|String|Len (Variables|Default|GetCurrent%20Code)) 4)
        (Variables|Default|SetCurrent%20Code "")))))

(event OnComponentBeginOverlap(Box_5)
  (params (OverlappedComponent :type Primitive%20Component%20Object%20Reference) (OtherActor :type Actor%20Object%20Reference) (OtherComp :type Primitive%20Component%20Object%20Reference) (OtherBodyIndex :type Integer) (bFromSweep :type Boolean) (SweepResult :type Hit%20Result%20Structure%20%28by%20ref%29))
  (bind _asvrpawn (Utilities|Casting|CastToVRPawn OtherActor))
  (if (== (Variables|/Game/VRTemplate/Blueprints/VRPawn.VRPawn_C|GetDetectZone _asvrpawn) OtherComp)
    (if (not (Variables|Default|GetTapped?))
      (Variables|Default|SetTapped? true)
      (CallFunction|Tap (Variables|Default|Get5))
      (Variables|Default|SetCurrent%20Code (Utilities|String|Append (Variables|Default|GetCurrent%20Code) "5"))
      (Audio|PlaySound2D "/Game/SND/Bip_Cue.Bip_Cue" 1.0 1.0 0.0 0 0)
      (CallFunction|Bip)
      (if (> (Utilities|String|Len (Variables|Default|GetCurrent%20Code)) 4)
        (Variables|Default|SetCurrent%20Code "")))))

(event OnComponentBeginOverlap(Box_9)
  (params (OverlappedComponent :type Primitive%20Component%20Object%20Reference) (OtherActor :type Actor%20Object%20Reference) (OtherComp :type Primitive%20Component%20Object%20Reference) (OtherBodyIndex :type Integer) (bFromSweep :type Boolean) (SweepResult :type Hit%20Result%20Structure%20%28by%20ref%29))
  (bind _asvrpawn (Utilities|Casting|CastToVRPawn OtherActor))
  (if (== (Variables|/Game/VRTemplate/Blueprints/VRPawn.VRPawn_C|GetDetectZone _asvrpawn) OtherComp)
    (if (not (Variables|Default|GetTapped?))
      (Variables|Default|SetTapped? true)
      (CallFunction|Tap (Variables|Default|Get9))
      (Variables|Default|SetCurrent%20Code (Utilities|String|Append (Variables|Default|GetCurrent%20Code) "9"))
      (Audio|PlaySound2D "/Game/SND/Bip_Cue.Bip_Cue" 1.0 1.0 0.0 0 0)
      (CallFunction|Bip)
      (if (> (Utilities|String|Len (Variables|Default|GetCurrent%20Code)) 4)
        (Variables|Default|SetCurrent%20Code "")))))

(event OnComponentBeginOverlap(Box_4)
  (params (OverlappedComponent :type Primitive%20Component%20Object%20Reference) (OtherActor :type Actor%20Object%20Reference) (OtherComp :type Primitive%20Component%20Object%20Reference) (OtherBodyIndex :type Integer) (bFromSweep :type Boolean) (SweepResult :type Hit%20Result%20Structure%20%28by%20ref%29))
  (bind _asvrpawn (Utilities|Casting|CastToVRPawn OtherActor))
  (if (== (Variables|/Game/VRTemplate/Blueprints/VRPawn.VRPawn_C|GetDetectZone _asvrpawn) OtherComp)
    (if (not (Variables|Default|GetTapped?))
      (Variables|Default|SetTapped? true)
      (CallFunction|Tap (Variables|Default|Get4))
      (Variables|Default|SetCurrent%20Code (Utilities|String|Append (Variables|Default|GetCurrent%20Code) "4"))
      (Audio|PlaySound2D "/Game/SND/Bip_Cue.Bip_Cue" 1.0 1.0 0.0 0 0)
      (CallFunction|Bip)
      (if (> (Utilities|String|Len (Variables|Default|GetCurrent%20Code)) 4)
        (Variables|Default|SetCurrent%20Code "")))))

(event OnComponentBeginOverlap(Box_3)
  (params (OverlappedComponent :type Primitive%20Component%20Object%20Reference) (OtherActor :type Actor%20Object%20Reference) (OtherComp :type Primitive%20Component%20Object%20Reference) (OtherBodyIndex :type Integer) (bFromSweep :type Boolean) (SweepResult :type Hit%20Result%20Structure%20%28by%20ref%29))
  (bind _asvrpawn (Utilities|Casting|CastToVRPawn OtherActor))
  (if (== (Variables|/Game/VRTemplate/Blueprints/VRPawn.VRPawn_C|GetDetectZone _asvrpawn) OtherComp)
    (if (not (Variables|Default|GetTapped?))
      (Variables|Default|SetTapped? true)
      (CallFunction|Tap (Variables|Default|Get3))
      (Variables|Default|SetCurrent%20Code (Utilities|String|Append (Variables|Default|GetCurrent%20Code) "3"))
      (Audio|PlaySound2D "/Game/SND/Bip_Cue.Bip_Cue" 1.0 1.0 0.0 0 0)
      (CallFunction|Bip)
      (if (> (Utilities|String|Len (Variables|Default|GetCurrent%20Code)) 4)
        (Variables|Default|SetCurrent%20Code "")))))

(event OnComponentBeginOverlap(Box_2)
  (params (OverlappedComponent :type Primitive%20Component%20Object%20Reference) (OtherActor :type Actor%20Object%20Reference) (OtherComp :type Primitive%20Component%20Object%20Reference) (OtherBodyIndex :type Integer) (bFromSweep :type Boolean) (SweepResult :type Hit%20Result%20Structure%20%28by%20ref%29))
  (bind _asvrpawn (Utilities|Casting|CastToVRPawn OtherActor))
  (if (== (Variables|/Game/VRTemplate/Blueprints/VRPawn.VRPawn_C|GetDetectZone _asvrpawn) OtherComp)
    (if (not (Variables|Default|GetTapped?))
      (Variables|Default|SetTapped? true)
      (CallFunction|Tap (Variables|Default|Get2))
      (Variables|Default|SetCurrent%20Code (Utilities|String|Append (Variables|Default|GetCurrent%20Code) "2"))
      (Audio|PlaySound2D "/Game/SND/Bip_Cue.Bip_Cue" 1.0 1.0 0.0 0 0)
      (CallFunction|Bip)
      (if (> (Utilities|String|Len (Variables|Default|GetCurrent%20Code)) 4)
        (Variables|Default|SetCurrent%20Code "")))))

(event OnComponentBeginOverlap(Box_1)
  (params (OverlappedComponent :type Primitive%20Component%20Object%20Reference) (OtherActor :type Actor%20Object%20Reference) (OtherComp :type Primitive%20Component%20Object%20Reference) (OtherBodyIndex :type Integer) (bFromSweep :type Boolean) (SweepResult :type Hit%20Result%20Structure%20%28by%20ref%29))
  (bind _asvrpawn (Utilities|Casting|CastToVRPawn OtherActor))
  (if (== (Variables|/Game/VRTemplate/Blueprints/VRPawn.VRPawn_C|GetDetectZone _asvrpawn) OtherComp)
    (if (not (Variables|Default|GetTapped?))
      (Variables|Default|SetTapped? true)
      (CallFunction|Tap (Variables|Default|Get1))
      (Variables|Default|SetCurrent%20Code (Utilities|String|Append (Variables|Default|GetCurrent%20Code) "1"))
      (Audio|PlaySound2D "/Game/SND/Bip_Cue.Bip_Cue" 1.0 1.0 0.0 0 0)
      (CallFunction|Bip)
      (if (> (Utilities|String|Len (Variables|Default|GetCurrent%20Code)) 4)
        (Variables|Default|SetCurrent%20Code "")))))

(event Custom|Tap
  (params (Target :type Scene%20Component%20Object%20Reference))
  (bind _relativelocation (Variables|/Script/Engine.SceneComponent|GetRelativeLocation Target))
  (Variables|Default|SetTapped? true)
  (Transformation|SetRelativeLocation Target (Math|Vector|MakeVector (Math|Float|Clamp(Float) (- (.x _relativelocation) 1.1) -1.1 0.0) (.y _relativelocation) (.z _relativelocation)) false false)
  (Utilities|FlowControl|Delay 0.1)
  (Transformation|SetRelativeLocation Target (Math|Vector|MakeVector (Math|Float|Clamp(Float) (- (.x _relativelocation) -1.1) -1.1 0.0) (.y _relativelocation) (.z _relativelocation)) false false)
  (Utilities|FlowControl|Delay 0.2)
  (Variables|Default|SetTapped? false))

(event Custom|CustomEvent_1
  (CallFunction|BadBip)
  (Audio|PlaySound2D "/Game/SND/Bip.Bip" 1.0 (* (Math|Conversions|ToFloat(Integer) (stale Custom|CustomEvent _result)) 0.3) 0.0 0 0))

(event Custom|ChooseCode
  (Variables|Default|SetCode%20To%20Solve (Utilities|String|Append (Utilities|String|Append (Utilities|String|ToString(Integer) (Math|Random|RandomIntegerinRange 0 9)) (Utilities|String|ToString(Integer) (Math|Random|RandomIntegerinRange 0 9))) (Utilities|String|Append (Utilities|String|ToString(Integer) (Math|Random|RandomIntegerinRange 0 9)) (Utilities|String|ToString(Integer) (Math|Random|RandomIntegerinRange 0 9))))))

(event Custom|Verify
  (if (Utilities|Enum|Equal(Enum) (Variables|Default|GetCode%20To%20Solve) (Variables|Default|GetCurrent%20Code))
    (Development|PrintString "Bueno")
    (Audio|PlaySound2D 0 1.0 1.0 0.0 0 0)
    (Variables|Default|SetCurrent%20Code "")
    (bind _returnvalue (Utilities|Time|SetTimerbyEvent (delegate Custom|CustomEvent) 0.7 true))
    (Variables|Default|SetNewVar_0 _returnvalue)
    (else
      (Development|PrintString "Pas Bueno")
      (Variables|Default|SetCurrent%20Code "")
      (Audio|PlaySound2D 0 1.0 1.0 0.0 0 0))))

(event Custom|CustomEvent
  (bind _result (Math|Integer|IncrementInt (Variables|Default|GetPitch))
    (:%20%20
      (if (>= _result 7)
        (Development|PrintString "Fin du game")
        (Utilities|Time|SetTimerbyEvent (delegate Custom|CustomEvent_1) 0.1 true)
        (Utilities|FlowControl|Delay 1.0)
        (Game|QuitGame 0 "Quit" false)
        (else
          (CallFunction|OsefBip)
          (Audio|PlaySound2D "/Game/SND/Bip.Bip" 1.0 (* (Math|Conversions|ToFloat(Integer) _result) 0.3) 0.0 0 0))))))

(event Custom|Bip
  (bind _bluespot (Variables|Default|GetBlueSpot))
  (Rendering|Components|Light|SetIntensity _bluespot 1e+05)
  (Utilities|FlowControl|Delay 0.05)
  (Rendering|Components|Light|SetIntensity _bluespot 0.0))

(event Custom|BadBip
  (bind _redspot (Variables|Default|GetRedSPot))
  (Rendering|Components|Light|SetIntensity _redspot 1e+05)
  (Utilities|FlowControl|Delay 0.05)
  (Rendering|Components|Light|SetIntensity _redspot 0.0))

(event Custom|OsefBip
  (bind _yellowspot (Variables|Default|GetYellowSpot))
  (Rendering|Components|Light|SetIntensity _yellowspot 1e+05)
  (Utilities|FlowControl|Delay 0.05)
  (Rendering|Components|Light|SetIntensity _yellowspot 0.0))

(event EventBeginPlay
  (|CallParentFunction)
  (CallFunction|ChooseCode)
  (Development|PrintString (Variables|Default|GetCode%20To%20Solve))
  (Rendering|Components|TextRender|SetText (Variables|Default|GetTextRender1) (Utilities|Text|ToText(String) (Variables|Default|GetCode%20To%20Solve))))

(event Collision|EventActorBeginOverlap
  (params (OtherActor :type Actor%20Object%20Reference))
  (|CallParentFunction OtherActor) ; This node is disabled and will not be called.\nDrag off pins to build functionality.
)

(event EventTick
  (params (DeltaSeconds :type Float%20%28single-precision%29))
  (|CallParentFunction DeltaSeconds) ; This node is disabled and will not be called.\nDrag off pins to build functionality.
)

(fn ConstructionScript
  (|CallParentFunction))

(fn VerifyBtnHit
  (params (Component%20Hitted :type Actor%20Component%20Object%20Reference) (Actor%20HItted :type Actor%20Object%20Reference))
  (bind _asvrpawn (Utilities|Casting|CastToVRPawn Actor%20HItted))
  (if (== (Variables|/Game/VRTemplate/Blueprints/VRPawn.VRPawn_C|GetDetectZone _asvrpawn) Component%20Hitted)
    (if (not (Variables|Default|GetTapped?))
      (Variables|Default|SetTapped? true)
      (return))))