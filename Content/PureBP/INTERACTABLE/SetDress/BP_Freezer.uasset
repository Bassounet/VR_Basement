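; BP_Freezer is an interactable set-dressing freezer whose lid swings open and closed.
; A look event briefly flags it interactable via a retriggerable delay, and the interact event toggles the lid only while flagged and not already moving.
; A timeline plays forward or in reverse, lerping the lid's relative rotation from its BeginPlay value by a configurable angle on a selectable axis.
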(event Custom|InteractDoor
  (bind _qngleforopen (Variables|Default|GetQngleForOpen))
  (bind _relative_rotation (Variables|Default|GetRelative%20Rotation))
  (bind _relative_rotation_2 (Variables|Default|GetRelative%20Rotation))
  (bind _relative_rotation_3 (Variables|Default|GetRelative%20Rotation))
  (if (not (Variables|Default|Getopen?))
    (Variables|Default|Setopen? true)
    (bind _newtrack_0 (Timeline|OpeningDoor PlayFromStart)
      (:Update
        (Variables|Default|Setmoving? true)
        (switch Utilities|FlowControl|Switch|SwitchonAxisRotate (Variables|Default|GetAXIS_ROTATE)
          (:NewEnumerator0
            (Transformation|SetRelativeRotation (Variables|Default|GetSM_Freezer_SM_Freezer_Lid) (Math|Rotator|MakeRotator (Math|Float|Lerp (.roll _relative_rotation) (+ (.roll _relative_rotation) _qngleforopen) _newtrack_0) (.pitch _relative_rotation) (.yaw _relative_rotation)) false false))
          (:NewEnumerator1
            (Transformation|SetRelativeRotation (Variables|Default|GetSM_Freezer_SM_Freezer_Lid) (Math|Rotator|MakeRotator (.roll _relative_rotation_3) (Math|Float|Lerp (.pitch _relative_rotation_3) (+ (.pitch _relative_rotation_3) _qngleforopen) _newtrack_0) (.yaw _relative_rotation_3)) false false))
          (:NewEnumerator2
            (Transformation|SetRelativeRotation (Variables|Default|GetSM_Freezer_SM_Freezer_Lid) (Math|Rotator|MakeRotator (.roll _relative_rotation_2) (.pitch _relative_rotation_2) (Math|Float|Lerp (.yaw _relative_rotation_2) (+ (.yaw _relative_rotation_2) _qngleforopen) _newtrack_0)) false false))))
      (:Finished
        (Variables|Default|Setmoving? false)))
    (else
      (Variables|Default|Setopen? false)
      (Timeline|OpeningDoor ReverseFromEnd))))

(event EventBeginPlay
  (Variables|Default|SetRelative%20Rotation (Variables|/Script/Engine.SceneComponent|GetRelativeRotation (Variables|Default|GetSM_Freezer_SM_Freezer_Lid))))

(event EventInterac
  (if (Variables|Default|GetInteractable)
    (if (not (Variables|Default|Getmoving?))
      (CallFunction|InteractDoor))))

(event EventLookingatYou
  (if (Variables|Default|GetInteractable)
    _
    (else
      (Variables|Default|SetInteractable true)))
  (Utilities|FlowControl|RetriggerableDelay 0.05)
  (Variables|Default|SetInteractable false))

(fn ConstructionScript)