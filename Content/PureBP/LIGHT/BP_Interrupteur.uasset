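; Interactable light switch that turns flickering on and off for BP_Flicker actors.
; On BeginPlay it builds its target list from all flickers, a preset list or those matching a group type, depending on Selection.
; Interacting plays a timeline forward or in reverse to roll the Axis, updates the text and notifies each target.
; Input stays locked until the animation finishes and flips the ON state.
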(event Custom|TurnON
  (bind _x_rot_base (Variables|Default|GetX_ROT_BASE))
  (bind _newtrack_0 (Timeline|TimelineForDescendingLOL PlayFromStart)
    (:Update
      (Transformation|SetWorldRotation (Variables|Default|GetAxis) (Math|Rotator|MakeRotator (Math|Float|Lerp _x_rot_base (+ _x_rot_base (Variables|Default|GetAngleRotationTrigger)) _newtrack_0) 0.0 0.0) false false))
    (:Finished
      (if (Variables|Default|GetON?)
        (Variables|Default|SetON? false)
        (else
          (Variables|Default|SetON? true)))
      (Variables|Default|SetInteractable? true))))

(event Custom|TurnOFF
  (bind _x_rot_base (Variables|Default|GetX_ROT_BASE))
  (bind _newtrack_0 (Timeline|TimelineForDescendingLOL ReverseFromEnd)
    (:Update
      (Transformation|SetWorldRotation (Variables|Default|GetAxis) (Math|Rotator|MakeRotator (Math|Float|Lerp _x_rot_base (+ _x_rot_base (Variables|Default|GetAngleRotationTrigger)) _newtrack_0) 0.0 0.0) false false))
    (:Finished
      (if (Variables|Default|GetON?)
        (Variables|Default|SetON? false)
        (else
          (Variables|Default|SetON? true)))
      (Variables|Default|SetInteractable? true))))

(event EventBeginPlay
  (Variables|Default|SetX_ROT_BASE (.roll (Transformation|GetWorldRotation (Variables|Default|GetAxis))))
  (switch Utilities|FlowControl|Switch|SwitchonInterrupteur_Choice (Variables|Default|GetSelection)
    (:NewEnumerator0
      (bind _outactors (Actor|GetAllActorsOfClass "/Game/PureBP/LIGHT/BP_Flicker.BP_Flicker_C"))
      (Variables|Default|SetTHE_Light _outactors))
    (:NewEnumerator1
      (Variables|Default|SetTHE_Light (Variables|Default|GetLight%20Affected)))
    (:NewEnumerator2
      (bind _outactors_2 (Actor|GetAllActorsOfClass "/Game/PureBP/LIGHT/BP_Flicker.BP_Flicker_C"))
      (for _array_element _outactors_2
        (if (Utilities|Enum|Equal(Enum) (Variables|/Game/PureBP/LIGHT/BP_Flicker.BP_Flicker_C|GetGROUPE_TYPE _array_element) (Variables|Default|GetGROUPE_TARGET))
          (Utilities|Array|Add (Variables|Default|GetTHE_Light) _array_element))))))

(event EventInterac
  (bind _the_light (Variables|Default|GetTHE_Light))
  (bind _textrender (Variables|Default|GetTextRender))
  (if (Variables|Default|GetInteractable?)
    (Components|Timeline|SetPlayRate (Variables|Default|GetTimelineForDescendingLOL) (/ 1.0 (Variables|Default|GetTimeForAnimation)))
    (Variables|Default|SetInteractable? false)
    (if (not (Variables|Default|GetON?))
      (CallFunction|TurnON)
      (Rendering|Components|TextRender|SetText _textrender (Variables|Default|GetValue))
      (for _array_element _the_light
        (Default|FlickeringON _array_element))
      (else
        (CallFunction|TurnOFF)
        (Rendering|Components|TextRender|SetText _textrender (Variables|Default|GetValue_0))
        (for _array_element_2 _the_light
          (Default|FlickeringOFF _array_element_2))))))

(fn ConstructionScript)