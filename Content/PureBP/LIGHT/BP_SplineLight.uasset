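; BP_SplineLight is an actor that strings lights along a spline and animates their visibility in LED-style patterns.
; The Construction Script adds a rect, spot or point light at each spline point except the last, hiding them for patterns that start dark.
; On BeginPlay, the chosen pattern starts a looping timer that steps an index through the lights, progressively switching them off or on, or moving a single dark or lit one along.
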(event Custom|ToLight_
  (bind _alllights (Variables|Default|GetAllLights))
  (if (< (+ (Variables|Default|GetLightIndex) 1) (Utilities|Array|Length _alllights))
    (Math|Integer|IncrementInt (Variables|Default|GetLightIndex) :!label _label
      (:%20%20
        (if (Utilities|IsValid (Utilities|Array|Get(acopy) _alllights (Variables|Default|GetLightIndex)))
          (Rendering|SetVisibility (Utilities|Array|Get(acopy) _alllights (Variables|Default|GetLightIndex)) true false))))
    (elif (Variables|Default|GetLooping?)
      (for _array_element (Variables|Default|GetAllLights)
        (Rendering|SetVisibility _array_element false false)
        (Variables|Default|SetLightIndex -2)
        (goto _label)))))

(event Custom|ToDark
  (bind _alllights (Variables|Default|GetAllLights))
  (if (<= (+ (Variables|Default|GetLightIndex) 1) (Utilities|Array|Length _alllights))
    (bind _result (Math|Integer|IncrementInt (Variables|Default|GetLightIndex) :!label _label)
      (:%20%20
        (if (Utilities|IsValid (Utilities|Array|Get(acopy) _alllights _result))
          (Rendering|SetVisibility (Utilities|Array|Get(acopy) _alllights _result) false false))))
    (else
      (Development|PrintString (Utilities|String|ToString(Integer) (Variables|Default|GetLightIndex)))
      (Variables|Default|SetLightIndex 0)
      (for _array_element _alllights
        (Rendering|SetVisibility _array_element true false)
        (goto _label)))))

(event Custom|oneLight
  (bind _alllights (Variables|Default|GetAllLights))
  (if (< (Variables|Default|GetLightIndex) (Utilities|Array|Length _alllights))
    (bind _result (Math|Integer|IncrementInt (Variables|Default|GetLightIndex) :!label _label)
      (:%20%20
        (if (Utilities|IsValid (Utilities|Array|Get(acopy) _alllights _result))
          (Rendering|SetVisibility (Utilities|Array|Get(acopy) _alllights _result) true false)
          (if (>= (- _result 1) 0)
            (if (Utilities|IsValid (Utilities|Array|Get(acopy) _alllights (- _result 1)))
              (Rendering|SetVisibility (Utilities|Array|Get(acopy) _alllights (- _result 1)) false false))))))
    (elif (Variables|Default|GetLooping?)
      (Variables|Default|SetLightIndex -2)
      (goto _label))))

(event Custom|TheFlickering
  (switch Utilities|FlowControl|Switch|SwitchonTypeLedFlickering (Variables|Default|GetLED%20Patern)
    (:NewEnumerator0
      (CallFunction|TODARK))
    (:NewEnumerator1
      (CallFunction|TOLIGHT))
    (:NewEnumerator2
      (CallFunction|ONELIGHT))
    (:NewEnumerator3
      (CallFunction|ONEDARK))))

(event Custom|TO_DARK
  (bind _returnvalue (Utilities|Time|SetTimerbyEvent (delegate Custom|ToDark) (Variables|Default|GetTime%20Beetween%20Lights) true))
  (Variables|Default|SetNewVar _returnvalue))

(event Custom|OneNight
  (bind _alllights (Variables|Default|GetAllLights))
  (if (< (Variables|Default|GetLightIndex) (Utilities|Array|Length _alllights))
    (bind _result (Math|Integer|IncrementInt (Variables|Default|GetLightIndex) :!label _label)
      (:%20%20
        (if (Utilities|IsValid (Utilities|Array|Get(acopy) _alllights _result))
          (Rendering|SetVisibility (Utilities|Array|Get(acopy) _alllights _result) false false)
          (if (Utilities|IsValid (Utilities|Array|Get(acopy) _alllights (- _result 1)))
            (Rendering|SetVisibility (Utilities|Array|Get(acopy) _alllights (- _result 1)) true false)))))
    (elif (Variables|Default|GetLooping?)
      (Variables|Default|SetLightIndex -1)
      (goto _label))))

(event Custom|ONE_DARK
  (bind _returnvalue (Utilities|Time|SetTimerbyEvent (delegate Custom|OneNight) (Variables|Default|GetTime%20Beetween%20Lights) true))
  (Variables|Default|SetNewVar _returnvalue))

(event Custom|ONE_LIGHT
  (bind _returnvalue (Utilities|Time|SetTimerbyEvent (delegate Custom|oneLight) (Variables|Default|GetTime%20Beetween%20Lights) true))
  (Variables|Default|SetNewVar _returnvalue))

(event Custom|TO_LIGHT
  (bind _returnvalue (Utilities|Time|SetTimerbyEvent (delegate Custom|ToLight_) (Variables|Default|GetTime%20Beetween%20Lights) true))
  (Variables|Default|SetNewVar _returnvalue))

(event EventBeginPlay
  (CallFunction|TheFlickering))

(fn ConstructionScript
  (bind _spline (Variables|Default|GetSpline))
  (bind _rotation (Variables|Default|GetRotation))
  (bind _alllights (Variables|Default|GetAllLights))
  (for _index (range 0 (- (Spline|GetNumberOfSplinePoints _spline) 2))
    (switch Utilities|FlowControl|Switch|SwitchonLightTypeCreated (Variables|Default|GetLightType)
      (:NewEnumerator0
        (bind _returnvalue (AddComponent|AddRectLightComponent false (Math|Transform|MakeTransform (.location (Math|Conversions|ToTransform(Vector) (Spline|GetLocationatSplinePoint _spline _index "Local"))) _rotation (.scale (Math|Conversions|ToTransform(Vector) (Spline|GetLocationatSplinePoint _spline _index "Local"))))))
        (Variables|Default|SetTheLightCreated _returnvalue))
      (:NewEnumerator1
        (bind _returnvalue_2 (AddComponent|AddSpotLightComponent false (Math|Transform|MakeTransform (.location (Math|Conversions|ToTransform(Vector) (Spline|GetLocationatSplinePoint _spline _index "Local"))) _rotation (.scale (Math|Conversions|ToTransform(Vector) (Spline|GetLocationatSplinePoint _spline _index "Local"))))))
        (Variables|Default|SetTheLightCreated _returnvalue_2))
      (:NewEnumerator2
        (bind _returnvalue_3 (AddComponent|AddPointLightComponent false (Math|Transform|MakeTransform (.location (Math|Conversions|ToTransform(Vector) (Spline|GetLocationatSplinePoint _spline _index "Local"))) _rotation (.scale (Math|Conversions|ToTransform(Vector) (Spline|GetLocationatSplinePoint _spline _index "Local"))))))
        (bind _output_get (Variables|Default|SetTheLightCreated _returnvalue_3))))
    (Utilities|Array|Add _alllights _output_get)
    (switch Utilities|FlowControl|Switch|SwitchonTypeLedFlickering (Variables|Default|GetLED%20Patern)
      (:NewEnumerator1
        _)
      (:NewEnumerator2
        _))
    (for _array_element _alllights
      (Rendering|SetVisibility _array_element false false))))