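; Flickering light actor that spawns a Rect, Spot or Point light and flickers while the first-person character's capsule is inside its trigger zone.
; Overlap starts a looping timer for Semi or Full flickering, which fade to random intensities with optional random colors, or Curve flickering, which replays a supplied float curve.
; The construction script builds a preview light, with helper functions to simulate, test and clean it in the editor.
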(event OnComponentBeginOverlap(ZoneTrigger)
  (params (OverlappedComponent :type Primitive%20Component%20Object%20Reference) (OtherActor :type Actor%20Object%20Reference) (OtherComp :type Primitive%20Component%20Object%20Reference) (OtherBodyIndex :type Integer) (bFromSweep :type Boolean) (SweepResult :type Hit%20Result%20Structure%20%28by%20ref%29))
  ;[1 1 1] TRIGGGER ZONE
  (Utilities|Casting|CastToBP_FirstPersonCharacter OtherActor)
  (Utilities|Casting|CastToCapsuleComponent OtherComp)
  (CallFunction|FlickeringON))

(event OnComponentEndOverlap(ZoneTrigger)
  (params (OverlappedComponent :type Primitive%20Component%20Object%20Reference) (OtherActor :type Actor%20Object%20Reference) (OtherComp :type Primitive%20Component%20Object%20Reference) (OtherBodyIndex :type Integer))
  ;[1 1 1] TRIGGGER ZONE
  (Utilities|Casting|CastToBP_FirstPersonCharacter OtherActor)
  (Utilities|Casting|CastToCapsuleComponent OtherComp)
  (CallFunction|FlickeringOFF))

(event Custom|FlickeringOFF
  ;[0 1 0.1554] ON/ OFF
  (Utilities|Time|ClearandInvalidateTimerbyHandle (Variables|Default|GetTimerFlicking))
  (Development|PrintString "OFF"))

(event Custom|FlickeringON
  ;[0 1 0.1554] ON/ OFF
  (CallFunction|Clignotage)
  (Development|PrintString "ON"))

(event Custom|CustomEvent
  ;[1 0.7095 0.0916] FLICKERING MANAGEMENT
  (Variables|Default|SetIntensityToModify (Variables|/Script/Engine.LightComponentBase|GetIntensity (Variables|Default|GetCurrentLight)))
  (Components|Timeline|SetPlayRate (Variables|Default|GetTimeForFade) (/ 1.0 (Math|Random|RandomFloatinRange (Variables|TimeForClignotage|GetMin_TimeClignot) (Variables|TimeForClignotage|GetMax_TimeClignot))))
  (Variables|Default|SetTargetIntensity (Math|Random|RandomFloatinRange (Variables|LightIntensity|GetMin%20Light%20Intensity) (Variables|LightIntensity|GetMax%20Light%20Intensity)))
  (bind _newtrack_0 (Timeline|TimeForFade PlayFromStart)
    (:Update
      (Rendering|Components|Light|SetIntensity (Variables|Default|GetCurrentLight) (Math|Float|Lerp (Variables|Default|GetIntensityToModify) (Variables|Default|GetTargetIntensity) _newtrack_0))
      ;[1 0 0] REDO
      (if (Variables|GENERAL|GetChangingColor?)
        (CallFunction|ColorManaging)))))

(event Custom|Clignotage
  (bind _min_light_intensity (Variables|LightIntensity|GetMin%20Light%20Intensity))
  (bind _max_light_intensity (Variables|LightIntensity|GetMax%20Light%20Intensity))
  (bind _returnvalue (Math|Random|RandomFloatinRange _min_light_intensity _max_light_intensity))
  (bind _returnvalue_2 (CallFunction|GetCurrentLight))
  ;[1 0.7095 0.0916] FLICKERING MANAGEMENT
  (Development|PrintString (Utilities|GetDisplayName _returnvalue_2))
  (switch Utilities|FlowControl|Switch|SwitchonTypeFlickering (Variables|GENERAL|GetFlickering_Type)
    (:NewEnumerator0
      (bind _returnvalue_3 (Utilities|Time|SetTimerbyEvent (delegate Custom|CustomEvent_1) (Math|Random|RandomFloatinRange (Variables|TimeForClignotage|GetMin_TimeClignot) (Variables|TimeForClignotage|GetMax_TimeClignot)) true))
      (Variables|Default|SetTimerFlicking _returnvalue_3))
    (:NewEnumerator1
      (bind _returnvalue_4 (Utilities|Time|SetTimerbyEvent (delegate Custom|CustomEvent) (Math|Random|RandomFloatinRange (Variables|TimeForClignotage|GetMin_TimeClignot) (Variables|TimeForClignotage|GetMax_TimeClignot)) true))
      (Variables|Default|SetTimerFlicking _returnvalue_4)
      (Rendering|Components|Light|SetIntensity (Variables|Default|GetCurrentLight) _returnvalue)
      ;[1 0 0] REDO
      (Development|PrintString (Utilities|String|ToString(Float) _returnvalue)))
    (:NewEnumerator2
      (CallFunction|Curving))))

(event Custom|ColorManaging
  (bind _new_light_color (Variables|ColorManaging|GetNew%20Light%20Color))
  ;[1 1 1] COLOR MANAGING
  (bind _returnvalue (CallFunction|GetCurrentLight))
  (if (and (Utilities|IsValid _returnvalue) (not (Utilities|Array|IsEmpty _new_light_color)))
    (Rendering|Components|Light|SetLightColor _returnvalue (Math|Conversions|ToLinearColor(Color) (Utilities|Array|Get(acopy) _new_light_color (Math|Random|RandomIntegerinRange 0 (- (Utilities|Array|Length _new_light_color) 1)))) true)))

(event Custom|CustomEvent_1
  ;[1 0.7095 0.0916] FLICKERING MANAGEMENT
  (Utilities|FlowControl|Delay (Math|Float|SelectFloat (Math|Random|RandomFloatinRange (Variables|SemiClignotage|GetMin%20Time%20Clignotage) (Variables|SemiClignotage|GetMax%20Time%20Clignotage)) (Variables|SemiClignotage|GetDelay%20Of%20Semi%20Clignotage) (Variables|Semi_Clignotage|GetRegular?)))
  (Variables|Default|SetIntensityToModify (Variables|/Script/Engine.LightComponentBase|GetIntensity (Variables|Default|GetCurrentLight)))
  (Components|Timeline|SetPlayRate (Variables|Default|GetTimeForFade) (/ 1.0 (Math|Random|RandomFloatinRange (Variables|TimeForClignotage|GetMin_TimeClignot) (Variables|TimeForClignotage|GetMax_TimeClignot))))
  (Variables|Default|SetTargetIntensity (Math|Random|RandomFloatinRange (Variables|LightIntensity|GetMin%20Light%20Intensity) (Variables|LightIntensity|GetMax%20Light%20Intensity)))
  (bind _newtrack_0 (Timeline|TimelineForSemiFade PlayFromStart)
    (:Update
      (Rendering|Components|Light|SetIntensity (Variables|Default|GetCurrentLight) (Math|Float|Lerp (Variables|Default|GetIntensityToModify) (Variables|Default|GetTargetIntensity) _newtrack_0))
      ;[1 0 0] REDO
      (if (Variables|GENERAL|GetChangingColor?)
        (CallFunction|ColorManaging)))))

(event Custom|CurvyFlickering
  ;[1 0.7095 0.0916] FLICKERING MANAGEMENT
  ;;[1 1 1] CURVING
  (bind _bp_flickercurve (Timeline|TimelineCurving PlayFromStart)
    (:Update
      (bind _returnvalue (CallFunction|GetCurrentLight))
      (Rendering|Components|Light|SetIntensity _returnvalue (* _bp_flickercurve (Variables|LightIntensity|GetMin%20Light%20Intensity))))))

(event Custom|Curving
  ;[1 0.7095 0.0916] FLICKERING MANAGEMENT
  ;;[1 1 1] CURVING
  (bind _returnvalue (Utilities|Time|SetTimerbyEvent (delegate Custom|CurvyFlickering) (.MaxTime (Math|Curves|GetTimeRange (Variables|Curve|GetTheCurve))) true 0.1))
  (Variables|Default|SetTimerFlicking _returnvalue))

(event EventBeginPlay
  (bind _componentcreated (Variables|Default|GetComponentCreated))
  (bind _arrow (Variables|Default|GetArrow))
  (bind _returnvalue (Transformation|GetRelativeTransform _arrow))
  ;[0.1354 0.1354 0.1354] LIGHT_CHOICE
  (switch Utilities|FlowControl|Switch|SwitchonLightTypeCreated (Variables|GENERAL|GetType%20Light%20To%20Create)
    (:NewEnumerator0
      (bind _returnvalue_2 (Game|AddComponentbyClass "/Script/Engine.RectLightComponent" false _returnvalue))
      (Variables|Default|SetRectCreated _returnvalue_2))
    (:NewEnumerator1
      (bind _returnvalue_3 (Game|AddComponentbyClass "/Script/Engine.SpotLightComponent" false _returnvalue))
      (Variables|Default|SetSpotCreated _returnvalue_3))
    (:NewEnumerator2
      (bind _returnvalue_4 (Game|AddComponentbyClass "/Script/Engine.PointLightComponent" false _returnvalue))
      (Variables|Default|SetPoint_Created _returnvalue_4)))
  (bind _returnvalue_5 (CallFunction|GetCurrentLight))
  (bind _output_get (Variables|Default|SetCurrentLight _returnvalue_5))
  (Rendering|Components|Light|SetIntensity _output_get (Variables|LightIntensity|GetMin%20Light%20Intensity))
  (Class|TimelineComponent|SetFloatCurve (Variables|Default|GetTimelineCurving) (Variables|Curve|GetTheCurve) "BP_FlickerCurve")
  (if (Utilities|IsValid _componentcreated)
    (Components|DestroyComponent _componentcreated)))

(event EventTick
  (params (DeltaSeconds :type Float%20%28single-precision%29)))

(fn ConstructionScript
  (bind _arrow (Variables|Default|GetArrow))
  (bind _returnvalue (Transformation|GetRelativeTransform _arrow))
  (Components|DestroyComponent (Variables|Default|GetComponentCreated))
  (switch Utilities|FlowControl|Switch|SwitchonLightTypeCreated (Variables|GENERAL|GetType%20Light%20To%20Create)
    (:NewEnumerator0
      (bind _returnvalue_2 (AddComponent|AddRectLightComponent false _returnvalue))
      (bind _output_get (Variables|Default|SetComponentCreated _returnvalue_2)))
    (:NewEnumerator1
      (bind _returnvalue_3 (AddComponent|AddSpotLightComponent false))
      (bind _output_get_2 (Variables|Default|SetComponentCreated _returnvalue_3)))
    (:NewEnumerator2
      (bind _returnvalue_4 (AddComponent|AddPointLightComponent false _returnvalue))
      (bind _output_get_3 (Variables|Default|SetComponentCreated _returnvalue_4))))
  (Rendering|Components|Light|SetIntensity _output_get (Variables|LightIntensity|GetMin%20Light%20Intensity)))

(fn SIMULATELIGHTS
  (bind _arrow (Variables|Default|GetArrow))
  (bind _returnvalue (Transformation|GetRelativeTransform _arrow))
  (if (not (Utilities|IsValid (Variables|Default|GetComponentCreated)))
    _
    (else
      (Components|DestroyComponent (Variables|Default|GetComponentCreated))))
  (switch Utilities|FlowControl|Switch|SwitchonLightTypeCreated (Variables|GENERAL|GetType%20Light%20To%20Create)
    (:NewEnumerator0
      (bind _returnvalue_2 (Game|AddComponentbyClass "/Script/Engine.RectLightComponent" false _returnvalue))
      (Variables|Default|SetComponentCreated _returnvalue_2))
    (:NewEnumerator1
      (bind _returnvalue_3 (Game|AddComponentbyClass "/Script/Engine.SpotLightComponent" false _returnvalue))
      (Variables|Default|SetComponentCreated _returnvalue_3))
    (:NewEnumerator2
      (bind _returnvalue_4 (Game|AddComponentbyClass "/Script/Engine.PointLightComponent" false _returnvalue))
      (Variables|Default|SetComponentCreated _returnvalue_4))))

(fn GetCurrentLight
  (bind _output_get (Variables|Default|SetCurrentLight (Variables|Default|GetComponentCreated)))
  (return _output_get))

(fn (SPAMME)FlickeringTest(SPAMME)
  (bind _componentcreated (Variables|Default|GetComponentCreated))
  (bind _new_light_color (Variables|ColorManaging|GetNew%20Light%20Color))
  (if (Utilities|IsValid _componentcreated)
    (Rendering|Components|Light|SetIntensity _componentcreated (Math|Random|RandomFloatinRange (Variables|LightIntensity|GetMin%20Light%20Intensity) (Variables|LightIntensity|GetMax%20Light%20Intensity)))
    (if (and (Utilities|IsValid _componentcreated) (not (Utilities|Array|IsEmpty _new_light_color)))
      (Rendering|Components|Light|SetLightColor _componentcreated (Math|Conversions|ToLinearColor(Color) (Utilities|Array|Get(acopy) _new_light_color (Math|Random|RandomIntegerinRange 0 (- (Utilities|Array|Length _new_light_color) 1)))) true))))

(fn CLEANLIGHTEDITORCREATED
  (bind _componentcreated (Variables|Default|GetComponentCreated))
  (if (Utilities|IsValid _componentcreated)
    (Components|DestroyComponent _componentcreated)))